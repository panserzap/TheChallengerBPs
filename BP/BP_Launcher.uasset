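; BP_Launcher is a launch pad that flings the first-person character when it overlaps the Box trigger.
; The launch velocity follows the Arrow component's forward vector scaled by Strength, overriding the character's existing horizontal and vertical velocity.
; A launch sound plays at the pad, then a second clip plays at the player's location after a short delay.
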(event `self.Box.OnComponentBeginOverlap`
  (params (OverlappedComponent :type "PrimitiveComponent Object Reference") (OtherActor :type "Actor Object Reference") (OtherComp :type "PrimitiveComponent Object Reference") (OtherBodyIndex :type Integer) (bFromSweep :type Boolean) (SweepResult :type "HitResult Structure (by ref)"))
  (bind _asfirst_person_character (cast `/Game/FirstPersonBP/Blueprints/FirstPersonCharacter` OtherActor))
  (set `self.PlayerRef` _asfirst_person_character)
  (`Character.LaunchCharacter` (`self.PlayerRef`) (* (`SceneComponent.GetForwardVector` (`self.Arrow`)) (`self.Strength`)) true true)
  (`GameplayStatics.PlaySoundAtLocation` "/Game/Audio/Launcher2.Launcher2" (`self.K2_GetActorLocation`) (struct) 1.0 1.0 0.0 null null null)
  (`KismetSystemLibrary.Delay` 1.0)
  (`GameplayStatics.PlaySoundAtLocation` "/Game/Audio/FlyYouFoolDarlek.FlyYouFoolDarlek" (`self.K2_GetActorLocation` (`GameplayStatics.GetPlayerCharacter` 0)) (struct) 1.0 1.0 0.0 null null null))

(fn `UserConstructionScript`)