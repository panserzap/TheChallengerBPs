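; BP_LetterExposal is a trigger actor that signals a letter to appear or disappear as the first-person character enters or leaves its box.
; Overlap begin and end fire the letter appear and disappear dispatchers with its LetterIndex.
; It starts hidden and non-colliding; Appear enables it with a teleport sound.
; The misspelled Dissapear event hides it again, while Disappear is empty.
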(event `Dissapear`
  (`self.SetActorEnableCollision` false)
  (`self.SetActorHiddenInGame` true))

(event `Disappear`)

(event `Appear`
  (`self.SetActorHiddenInGame` false)
  (`self.SetActorEnableCollision` true)
  (`GameplayStatics.PlaySoundAtLocation` "/Engine/VREditor/Sounds/UI/Teleport_Mode_Entered.Teleport_Mode_Entered" (`self.K2_GetActorLocation`) (struct) 1.0 1.0 0.0 null null null))

(event `self.BoxCollision.OnComponentBeginOverlap`
  (params (OverlappedComponent :type "PrimitiveComponent Object Reference") (OtherActor :type "Actor Object Reference") (OtherComp :type "PrimitiveComponent Object Reference") (OtherBodyIndex :type Integer) (bFromSweep :type Boolean) (SweepResult :type "HitResult Structure (by ref)"))
  (cast `/Game/FirstPersonBP/Blueprints/FirstPersonCharacter` OtherActor)
  (`self.LetterAppearDispatcher` (`self.LetterIndex`)))

(event `self.BoxCollision.OnComponentEndOverlap`
  (params (OverlappedComponent :type "PrimitiveComponent Object Reference") (OtherActor :type "Actor Object Reference") (OtherComp :type "PrimitiveComponent Object Reference") (OtherBodyIndex :type Integer))
  (cast `/Game/FirstPersonBP/Blueprints/FirstPersonCharacter` OtherActor)
  (`self.LetterDisappearDispatcher` (`self.LetterIndex`)))

(fn `UserConstructionScript`
  (`self.SetActorHiddenInGame` true)
  (`self.SetActorEnableCollision` false))