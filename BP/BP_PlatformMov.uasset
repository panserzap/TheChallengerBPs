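; BP_PlatformMov is a moving platform actor whose static mesh travels along a spline.
; Custom events start and stop three timelines: basic movement, slow reverse and fast reverse.
; Each timeline scales its DistanceTraveled track by spline length to set the mesh's world location, without sweep.
; Movement restarts from the beginning, while both reverse variants resume from their current position; nothing in this Blueprint calls these events.
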(event `Movement`
  (bind (_direction _distancetraveled) (`Timeline|Timeline_0` :!via `PlayFromStart` :!label _label)
    (:`Update`
      (`SceneComponent.K2_SetWorldLocation` (`self.StaticMesh`) (`SplineComponent.GetLocationAtDistanceAlongSpline` (`self.Spline`) (* _distancetraveled (`SplineComponent.GetSplineLength` (`self.Spline`))) "World") false false))))

(event `Stop`
  (goto _label :!via `Stop`))

(event `ReverseSlow`
  (bind (_direction _distancetraveled) (`Timeline|TimeLineWithRevers` :!label _label_2)
    (:`Update`
      (`SceneComponent.K2_SetWorldLocation` (`self.StaticMesh`) (`SplineComponent.GetLocationAtDistanceAlongSpline` (`self.Spline`) (* _distancetraveled (`SplineComponent.GetSplineLength` (`self.Spline`))) "World") false false))))

(event `StopReverseSlow`
  (goto _label_2 :!via `Stop`))

(event `ReverseFast`
  (bind (_direction _distancetraveled) (`Timeline|Timeline_1` :!label _label_3)
    (:`Update`
      (`SceneComponent.K2_SetWorldLocation` (`self.StaticMesh`) (`SplineComponent.GetLocationAtDistanceAlongSpline` (`self.Spline`) (* _distancetraveled (`SplineComponent.GetSplineLength` (`self.Spline`))) "World") false false))))

(event `StopReverseFast`
  (goto _label_3 :!via `Stop`))

(fn `UserConstructionScript`)