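; Actor component that gives the first-person character a directional dash ability.
; ActivateAbility launches the character along its current velocity, or along its forward vector when standing still, using separate force multipliers.
; After a duration scaled by global time dilation, it halts movement and plays the dash sound.
; An active flag and the character's CanDash flag block dashing until a short cooldown ends.
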(event `ActivateAbility`
  (bind _character (`self.Character`))
  (bind _velocity (`MovementComponent.Velocity` (`Character.CharacterMovement` (`self.Character`))))
  ;[0 0 0 0.5] Dash
  (bind _asfirst_person_character (cast `/Game/FirstPersonBP/Blueprints/FirstPersonCharacter` (`self.GetOwner`)))
  (bind _output_get (set `self.Character` _asfirst_person_character))
  (set `/Game/FirstPersonBP/Blueprints/FirstPersonCharacter.CanDash` false _output_get)
  (if (not (`self.IsDashActive?`))
    (set `self.IsDashActive?` true)
    (if (== (`KismetMathLibrary.VSize` _velocity) 0.0)
      (`Character.LaunchCharacter` (`self.Character`) (* (`Actor.GetActorForwardVector` (`self.Character`)) (`self.ForceMultiplierStill`)) true true)
      (else
        (`Character.LaunchCharacter` (`self.Character`) (* _velocity (`self.ForceMultiplier`)) true true)))
    (`KismetSystemLibrary.Delay` (* (`self.DashDuration`) (`GameplayStatics.GetGlobalTimeDilation`)))
    (`MovementComponent.StopMovementImmediately` (`Character.CharacterMovement` _character))
    (`GameplayStatics.PlaySoundAtLocation` "/Game/Audio/DashSound.DashSound" (`Actor.K2_GetActorLocation` _character) (struct) 1.0 1.0 0.0 null null null)
    (`KismetSystemLibrary.Delay` 0.5)
    (set `self.IsDashActive?` false)
    (set `/Game/FirstPersonBP/Blueprints/FirstPersonCharacter.CanDash` true (`self.Character`))))