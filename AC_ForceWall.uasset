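; Actor component for a force wall/prison ability that spawns a BP_ForceWall where the owning first-person character is aiming.
; ActivateAbility line traces from the camera up to ShieldDistance, placing the wall at the hit point or trace end.
; The wall takes the camera's yaw and roll but not its pitch.
; Spawning is blocked while the previous wall still exists or the delay-based cooldown flag is set.
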(event `ActivateAbility`
  (bind (_returnvalue_roll _returnvalue_pitch _returnvalue_yaw) (`KismetMathLibrary.BreakRotator` (`SceneComponent.K2_GetComponentRotation` (`self.Camera`))))
  (bind _firstpersoncamera (`/Game/FirstPersonBP/Blueprints/FirstPersonCharacter.FirstPersonCamera` (`self.Character`)))
  (bind _returnvalue (`SceneComponent.K2_GetComponentLocation` _firstpersoncamera))
  ;[1 1 1] Force Wall/Prison
  (bind _asfirst_person_character (cast `/Game/FirstPersonBP/Blueprints/FirstPersonCharacter` (`self.GetOwner`)))
  (set `self.Character` _asfirst_person_character)
  (bind _firstpersoncamera_2 (`/Game/FirstPersonBP/Blueprints/FirstPersonCharacter.FirstPersonCamera` _asfirst_person_character))
  (`/Engine/EditorBlueprintResources/StandardMacros.IsValid` _firstpersoncamera_2
    (:`Is Valid`
      (set `self.Camera` _firstpersoncamera_2)
      ;;[1 1 1] shieldchecks
      (`/Engine/EditorBlueprintResources/StandardMacros.IsValid` (`self.ShieldActorRef`)
        (:`Is Not Valid`
          (if (not (`self.ShieldCoolDown?`))
            (set `self.ShieldCoolDown?` true)
            (`/Engine/EditorBlueprintResources/StandardMacros.IsValid` _firstpersoncamera
              (:`Is Valid`
                (bind (_outhit _returnvalue_2) (`KismetSystemLibrary.LineTraceSingle` _returnvalue (+ _returnvalue (* (`SceneComponent.GetForwardVector` _firstpersoncamera) (`self.ShieldDistance`))) "TraceTypeQuery1"))
                (if _returnvalue_2
                  (bind (_bblockinghit _binitialoverlap _time _distance _location _impactpoint _normal _impactnormal _physmat _hitactor _hitcomponent _hitbonename _hititem _faceindex _tracestart _traceend) (`GameplayStatics.BreakHitResult` _outhit))
                  (set `self.HitLocation` _location)
                  (else
                    (set `self.HitLocation` _traceend)))
                (bind _returnvalue_3 (`|SpawnActorFromClass` "/Game/Blueprints/BP_ForceWall.BP_ForceWall_C" (`KismetMathLibrary.MakeTransform` (`self.HitLocation`) (`KismetMathLibrary.MakeRotator` _returnvalue_roll 0.0 _returnvalue_yaw)) "Undefined" "OverrideRootScale" null null))
                (set `self.ShieldActorRef` _returnvalue_3)
                (`KismetSystemLibrary.Delay` (`self.ShieldCoolDown`))
                (set `self.ShieldCoolDown?` false)))))))))